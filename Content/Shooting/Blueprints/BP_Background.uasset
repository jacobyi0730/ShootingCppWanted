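; BP_Background is a background mesh actor in the Shooting folder that sets a material scroll speed from keyboard input.
; On BeginPlay it creates a dynamic instance of its mesh material and enables input for the first player controller.
; Key 1 sets ScrollSpeed on that instance, while key 2 sets the same-named vector in the MPC_Background parameter collection, contrasting per-instance and collection-wide control.
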(event EventBeginPlay
  (bind _staticmeshcomponent (Variables|Debug|GetStaticMeshComponent))
  (bind _returnvalue (Rendering|Material|CreateDynamicMaterialInstance _staticmeshcomponent 0 (Rendering|Material|GetMaterial _staticmeshcomponent 0) "None" :!class /Script/Engine.PrimitiveComponent))
  (Variables|Default|SetMat _returnvalue)
  (Input|EnableInput (Game|GetPlayerController 0)))

(event Collision|EventActorBeginOverlap
  (params (OtherActor :type Actor%20Object%20Reference)))

(event EventTick
  (params (DeltaSeconds :type Float%20%28single-precision%29)))

(event Input|KeyboardEvents|1
  (params (Key :type Key%20Structure :default "None"))
  (:Pressed
    (Rendering|Material|SetVectorParameterValue (Variables|Default|GetMat) "ScrollSpeed" (Utilities|Struct|MakeLinearColor 0.0 -1.0 0.0 0.0) :!class /Script/Engine.MaterialInstanceDynamic)))

(event Input|KeyboardEvents|2
  (params (Key :type Key%20Structure :default "None"))
  (:Pressed
    (Rendering|Material|SetVectorParameterValue "/Game/Shooting/Blueprints/MPC_Background.MPC_Background" "ScrollSpeed" (Utilities|Struct|MakeLinearColor 0.0 -1.0 0.0 0.0) :!class /Script/Engine.KismetMaterialLibrary)))

(fn ConstructionScript)