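; Game mode for the shooting game that persists the player's high score through a save game slot.
; BlueprintLoadGame reads the high score from an existing BP_SaveGame slot into HighScore.
; BlueprintSaveGame writes the passed score to a fresh save object in that slot, without comparing it or updating HighScore.
; BeginPlay is empty, so neither function is called within this graph.
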(event EventBeginPlay)

(event EventTick
  (params (DeltaSeconds :type Float%20%28single-precision%29)))

(fn ConstructionScript)

(fn BlueprintLoadGame
  (bind _returnvalue (SaveGame|DoesSaveGameExist "SaveGameData"))
  (if _returnvalue
    (bind _returnvalue_2 (SaveGame|LoadGamefromSlot "SaveGameData"))
    (bind _asbp_save_game (Utilities|Casting|CastToBP_SaveGame _returnvalue_2))
    (Variables|Default|SetHighScore (Variables|/Game/Shooting/Blueprints/BP_SaveGame.BP_SaveGame_C|GetSave_HighScore _asbp_save_game))))

(fn BlueprintSaveGame
  (params (NewHighScore :type Integer))
  (bind _returnvalue (SaveGame|CreateSaveGameObject "/Game/Shooting/Blueprints/BP_SaveGame.BP_SaveGame_C"))
  (LocalVariables|SetSaveGameInstance _returnvalue)
  (Variables|/Game/Shooting/Blueprints/BP_SaveGame.BP_SaveGame_C|SetSave_HighScore (LocalVariables|GetSaveGameInstance) NewHighScore)
  (SaveGame|SaveGametoSlot (LocalVariables|GetSaveGameInstance) "SaveGameData"))